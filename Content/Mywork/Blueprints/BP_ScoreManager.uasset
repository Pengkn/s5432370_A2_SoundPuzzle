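; Score manager that counts correct and incorrect answers and persists a high score for each.
; BeginPlay loads both records from a BP_SaveManager save slot, defaulting to zero if none exists.
; Each increment that meets or beats its record immediately loads or creates the save object and writes it back.
; ResetScore only deletes the slot, leaving in-memory values intact; SavingRightHighScore is an unused duplicate of SavingRightHighScore2.
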(event `Update Score`
  ; save highscore
  (bind _returnvalue (`GameplayStatics.DoesSaveGameExist` (`self.Save Slot Name `)))
  (if _returnvalue
    (bind _returnvalue_2 (`GameplayStatics.LoadGameFromSlot` (`self.Save Slot Name `)))
    (bind _output_get (set `self.SaverSubClass` _returnvalue_2))
    (bind _asbp_save_manager (cast `/Game/Mywork/Blueprints/BP_SaveManager` _output_get))
    (set `self.HighScoreRight` (`/Game/Mywork/Blueprints/BP_SaveManager.HighScoreRight` _asbp_save_manager))
    (set `self.HighScoreWrong` (`/Game/Mywork/Blueprints/BP_SaveManager.HighScoreWrong` _asbp_save_manager))
    (else
      (set `self.HighScoreRight` 0)
      (set `self.HighScoreWrong` 0))))

(event `AddScore_Correct`
  ;[0.07798 0.15 0.06278 0.5] Score Management
  (set `self.ScoreRight` (+ (`self.ScoreRight`) 1))
  (`self.Saving Right High Score2`))

(event `ResetScore`
  ; reset score mechanic
  (`GameplayStatics.DeleteGameInSlot` (`self.Save Slot Name `)))

(event `self.ReceiveBeginPlay`
  (`self.Update Score`))

(event `AddScore_Incorrect`
  ;[0.07798 0.15 0.06278 0.5] Score Management
  (set `self.ScoreWrong` (+ (`self.ScoreWrong`) 1))
  (`self.Saving Wrong High Score`))

(fn `Saving Right High Score`
  (if (>= (`self.ScoreRight`) (`self.HighScoreRight`))
    (bind _output_get (set `self.HighScoreRight` (`self.ScoreRight`)))
    (bind _returnvalue (`GameplayStatics.DoesSaveGameExist` (`self.Save Slot Name `)))
    (if _returnvalue
      (bind _returnvalue_2 (`GameplayStatics.LoadGameFromSlot` (`self.Save Slot Name `)))
      (bind _output_get_2 (set `self.SaverSubClass` _returnvalue_2))
      (bind _asbp_save_manager (cast `/Game/Mywork/Blueprints/BP_SaveManager` _output_get_2))
      (set `/Game/Mywork/Blueprints/BP_SaveManager.HighScoreRight` _output_get _asbp_save_manager)
      (`GameplayStatics.SaveGameToSlot` (`self.SaverSubClass`) (`self.Save Slot Name `))
      (else
        (bind _returnvalue_3 (`GameplayStatics.CreateSaveGameObject` "/Game/Mywork/Blueprints/BP_SaveManager.BP_SaveManager_C"))
        (bind _output_get_3 (set `self.SaverSubClass` _returnvalue_3))
        (bind _asbp_save_manager_2 (cast `/Game/Mywork/Blueprints/BP_SaveManager` _output_get_3))
        (set `/Game/Mywork/Blueprints/BP_SaveManager.HighScoreRight` _output_get _asbp_save_manager_2)
        (`GameplayStatics.SaveGameToSlot` (`self.SaverSubClass`) (`self.Save Slot Name `))))))

(fn `Saving Right High Score2`
  (if (>= (`self.ScoreRight`) (`self.HighScoreRight`))
    (bind _output_get (set `self.HighScoreRight` (`self.ScoreRight`)))
    (bind _returnvalue (`GameplayStatics.DoesSaveGameExist` (`self.Save Slot Name `)))
    (if _returnvalue
      (bind _returnvalue_2 (`GameplayStatics.LoadGameFromSlot` (`self.Save Slot Name `)))
      (bind _output_get_2 (set `self.SaverSubClass` _returnvalue_2))
      (bind _asbp_save_manager (cast `/Game/Mywork/Blueprints/BP_SaveManager` _output_get_2))
      (set `/Game/Mywork/Blueprints/BP_SaveManager.HighScoreRight` _output_get _asbp_save_manager)
      (`GameplayStatics.SaveGameToSlot` _output_get_2 (`self.Save Slot Name `))
      (else
        (bind _returnvalue_3 (`GameplayStatics.CreateSaveGameObject` "/Game/Mywork/Blueprints/BP_SaveManager.BP_SaveManager_C"))
        (bind _output_get_3 (set `self.SaverSubClass` _returnvalue_3))
        (bind _asbp_save_manager_2 (cast `/Game/Mywork/Blueprints/BP_SaveManager` _output_get_3))
        (set `/Game/Mywork/Blueprints/BP_SaveManager.HighScoreRight` _output_get _asbp_save_manager_2)
        (`GameplayStatics.SaveGameToSlot` _output_get_3 (`self.Save Slot Name `))))))

(fn `Saving Wrong High Score`
  (if (>= (`self.ScoreWrong`) (`self.HighScoreWrong`))
    (bind _output_get (set `self.HighScoreWrong` (`self.ScoreWrong`)))
    (bind _returnvalue (`GameplayStatics.DoesSaveGameExist` (`self.Save Slot Name `)))
    (if _returnvalue
      (bind _returnvalue_2 (`GameplayStatics.LoadGameFromSlot` (`self.Save Slot Name `)))
      (bind _output_get_2 (set `self.SaverSubClass` _returnvalue_2))
      (bind _asbp_save_manager (cast `/Game/Mywork/Blueprints/BP_SaveManager` _output_get_2))
      (set `/Game/Mywork/Blueprints/BP_SaveManager.HighScoreWrong` _output_get _asbp_save_manager)
      (`GameplayStatics.SaveGameToSlot` _output_get_2 (`self.Save Slot Name `))
      (else
        (bind _returnvalue_3 (`GameplayStatics.CreateSaveGameObject` "/Game/Mywork/Blueprints/BP_SaveManager.BP_SaveManager_C"))
        (bind _output_get_3 (set `self.SaverSubClass` _returnvalue_3))
        (bind _asbp_save_manager_2 (cast `/Game/Mywork/Blueprints/BP_SaveManager` _output_get_3))
        (set `/Game/Mywork/Blueprints/BP_SaveManager.HighScoreWrong` _output_get _asbp_save_manager_2)
        (`GameplayStatics.SaveGameToSlot` _output_get_3 (`self.Save Slot Name `))))))

(fn `UserConstructionScript`)