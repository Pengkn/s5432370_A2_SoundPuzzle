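; HUD manager Blueprint that creates the WBP_HUD widget on BeginPlay and shows timed HUD text and subtitles.
; SetHUDtextVisibility clears the HUD text, then shows the Target element for two seconds.
; ShowSubtitleText hides all subtitles, then switches between Typing, Manual Override and Door Open widgets for a brief display.
; A DoOnce resets after each display, so requests arriving meanwhile hide the current subtitle without showing another.
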(event `self.ReceiveBeginPlay`
  (bind _returnvalue (`|CreateWidget` "/Game/Mywork/Blueprints/UI/WBP_HUD.WBP_HUD_C"))
  (bind _output_get (set `self.HUD_Ref` _returnvalue))
  (`UserWidget.AddToViewport` _output_get 0))

(event `SetHUDtextVisibility`
  (bind _target (`/Game/Mywork/Blueprints/UI/WBP_HUD.Target` (`self.HUD_Ref`)))
  (`/Game/Mywork/Blueprints/UI/WBP_HUD.Hide all HUD Text` (`self.HUD_Ref`))
  (set `Widget.Visibility` "Visible" _target)
  (`KismetSystemLibrary.Delay` 2.0)
  (set `Widget.Visibility` "Hidden" _target)
  (`/Game/Mywork/Blueprints/UI/WBP_HUD.Hide all HUD Text` (`self.HUD_Ref`)))

(event `SetSubtitleTextVisibility`
  (params (`Subtitle Input` :type "Widget Object Reference"))
  (`/Engine/EditorBlueprintResources/StandardMacros.DoOnce` false :!label _label
    (:`Completed`
      (set `Widget.Visibility` "Visible" `Subtitle Input`)
      (`KismetSystemLibrary.Delay` 1.5)
      (set `Widget.Visibility` "Hidden" `Subtitle Input`)
      (`self.Hide All Subtitles`)
      (goto _label :!via `Reset`))))

(event `Hide All Subtitles`
  (bind _hud_ref (`self.HUD_Ref`))
  (set `Widget.Visibility` "Hidden" (`/Game/Mywork/Blueprints/UI/WBP_HUD.WBP_Text_Base_Typing` _hud_ref))
  (set `Widget.Visibility` "Hidden" (`/Game/Mywork/Blueprints/UI/WBP_HUD.WBP_Text_Base_ManualOverride` _hud_ref))
  (set `Widget.Visibility` "Hidden" (`/Game/Mywork/Blueprints/UI/WBP_HUD.WBP_Text_Base_DoorOpen` _hud_ref)))

(event `Show Subtitle Text`
  (params (`Subtitle Text` :type "/Game/Mywork/Blueprints/UI/E_Subtitle_Text Enum" :default "NewEnumerator0"))
  (bind _hud_ref (`self.HUD_Ref`))
  (`self.Hide All Subtitles`)
  (switch `/Game/Mywork/Blueprints/UI/E_Subtitle_Text` `Subtitle Text`
    (:`NewEnumerator0`
      (`self.SetSubtitleTextVisibility` (`/Game/Mywork/Blueprints/UI/WBP_HUD.WBP_Text_Base_Typing` _hud_ref)))
    (:`NewEnumerator1`
      (`self.SetSubtitleTextVisibility` (`/Game/Mywork/Blueprints/UI/WBP_HUD.WBP_Text_Base_ManualOverride` _hud_ref)))
    (:`NewEnumerator2`
      (`self.SetSubtitleTextVisibility` (`/Game/Mywork/Blueprints/UI/WBP_HUD.WBP_Text_Base_DoorOpen` _hud_ref)))))

(fn `UserConstructionScript`)