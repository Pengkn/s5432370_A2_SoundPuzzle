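; Interactable sound button for a sequence puzzle, triggered through Interact while the first-person character is in range.
; A sphere overlap toggles the interaction widget, screen prompt and custom-depth outline.
; A valid press animates the mesh, shakes the camera, plays its track and registers its ID with the puzzle manager, which holds a shared cooldown; blocked presses show HUD text.
; PlayButtonSoundOnly plays the track with a subtitle for sequence playback.
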(event `Animate Button`
  ; Button Animation
  (if (`/Game/Mywork/Blueprints/BP_PuzzleManager.AcceptingPlayerInput` (`self.PuzzleManagerREf`))
    (bind (_direction _button_scale) (`Timeline|Button Animation` :!label _label)
      (:`Update`
        (`SceneComponent.SetRelativeScale3D` (`self.ButtonMesh`) _button_scale)
        (`KismetSystemLibrary.Delay` 0.5)
        (goto _label :!via `Reverse`)))))

(event `/Game/Mywork/Blueprints/BPI_Interaction.OnInteractionRangeEntered`
  ;[0.1267 0.15 0.03227 0.5] Interact Widget UI and Interact Outline
  (set `self.CloseEnough?` true)
  (`SceneComponent.SetHiddenInGame` (`self.Interaction Widget`) false true))

(event `self.Sphere.OnComponentBeginOverlap`
  (params (OverlappedComponent :type "PrimitiveComponent Object Reference") (OtherActor :type "Actor Object Reference") (OtherComp :type "PrimitiveComponent Object Reference") (OtherBodyIndex :type Integer) (bFromSweep :type Boolean) (SweepResult :type "HitResult Structure (by ref)"))
  ;[0.1267 0.15 0.03227 0.5] Interact Widget UI and Interact Outline
  (cast `/Game/Mywork/Blueprints/BP_FirstPersonCharacter` OtherActor)
  (`self.OnInteractionRangeEntered`)
  (`UserWidget.AddToViewport` (`self.InteractPrompt`) 0)
  (`PrimitiveComponent.SetRenderCustomDepth` (`self.ButtonMesh`) true))

(event `/Game/Mywork/Blueprints/BPI_Interaction.OnInteractionRangeExited`
  ;[0.1267 0.15 0.03227 0.5] Interact Widget UI and Interact Outline
  (set `self.CloseEnough?` false)
  (`SceneComponent.SetHiddenInGame` (`self.Interaction Widget`) true true))

(event `self.Sphere.OnComponentEndOverlap`
  (params (OverlappedComponent :type "PrimitiveComponent Object Reference") (OtherActor :type "Actor Object Reference") (OtherComp :type "PrimitiveComponent Object Reference") (OtherBodyIndex :type Integer))
  ;[0.1267 0.15 0.03227 0.5] Interact Widget UI and Interact Outline
  (cast `/Game/Mywork/Blueprints/BP_FirstPersonCharacter` OtherActor)
  (`self.OnInteractionRangeExited`)
  (`Widget.RemoveFromParent` (`self.InteractPrompt`))
  (`PrimitiveComponent.SetRenderCustomDepth` (`self.ButtonMesh`) false))

(event `self.ReceiveBeginPlay`
  ;[0.1267 0.15 0.03227 0.5] Interact Widget UI and Interact Outline
  (bind _returnvalue (`|CreateWidget` "/Game/Mywork/UI/WBP_InteractPrompt.WBP_InteractPrompt_C"))
  (set `self.InteractPrompt` _returnvalue)
  (bind _aswbp_interaction (cast `/Game/Mywork/UI/WBP_Interaction` (`WidgetComponent.GetUserWidgetObject` (`self.Interaction Widget`))))
  (set `/Game/Mywork/UI/WBP_Interaction.Text Content` (`self.SoundWidgetText`) _aswbp_interaction))

(event `UseButton`
  (bind _puzzlemanagerref (`self.PuzzleManagerREf`))
  (bind _audio (`self.Audio`))
  (bind _hudmanagerref (`self.HUDmanagerref`))
  ;[0.02234 0.08376 0.15 0.5] Player Button & Sound Input:
  (if (`self.CloseEnough?`)
    (if (`/Game/Mywork/Blueprints/BP_PuzzleManager.AcceptingPlayerInput` (`self.PuzzleManagerREf`))
      (if (`/Game/Mywork/Blueprints/BP_PuzzleManager.CanUseNextButton?` _puzzlemanagerref)
        (set `/Game/Mywork/Blueprints/BP_PuzzleManager.CanUseNextButton?` false _puzzlemanagerref)
        (`self.Animate Button`)
        (`GameplayStatics.PlayWorldCameraShake` "/Game/Mywork/Blueprints/BP_CameraShake.BP_CameraShake_C" (`self.K2_GetActorLocation`) 0.0 200.0)
        (`AudioComponent.SetSound` _audio (`|GetArrayItem` (`self.Tracks`) (`self.Track Index`)))
        (`AudioComponent.Play` _audio 0.0)
        (`/Game/Mywork/Blueprints/BP_PuzzleManager.RegisterPlayerInput` (`self.PuzzleManagerREf`) (`self.ButtonID`))
        (`KismetSystemLibrary.Delay` 2.5)
        (set `/Game/Mywork/Blueprints/BP_PuzzleManager.CanUseNextButton?` true (`self.PuzzleManagerREf`))
        (else
          (`/Game/Mywork/UI/WBP_HUD.set enum` (`/Game/Mywork/Blueprints/BP_HUDManager.HUD_Ref` _hudmanagerref) "NewEnumerator1" :!label _label_2)
          (`/Game/Mywork/Blueprints/BP_HUDManager.SetHUDtextVisibility` _hudmanagerref)))
      (else
        (goto _label_2)))))

(event `PlayButtonSoundOnly`
  (bind _audio (`self.Audio`))
  ;[0.15 0 0.0121 0.5] Generates corresponding sounds for correct sequence:
  (`/Game/Mywork/Blueprints/BP_HUDManager.Show Subtitle Text` (`self.HUDmanagerref`) (`self.Subtitle text`))
  (`AudioComponent.SetSound` _audio (`|GetArrayItem` (`self.Tracks`) (`self.Track Index`)))
  (`AudioComponent.Play` _audio 0.0))

(fn `Interact`
  (params (Interactor :type "Character Object Reference"))
  (returns (Sucess :type Boolean))
  (`self.UseButton`)
  (return true))

(fn `UserConstructionScript`)