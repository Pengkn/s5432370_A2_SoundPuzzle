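; BP_WinCondition is a trigger actor that ends the game in a win when something overlaps its Box component.
; The overlap fires WinCondition, which adds a WBP_WinMenu widget, shows the cursor, switches to UI-only input and pauses the game.
; The player-character check is left unconnected, so any overlapping actor triggers the win.
; Input focus targets WIDWinMenuRef, which the graph never assigns from the created widget.
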(event `self.Box.OnComponentBeginOverlap`
  (params (OverlappedComponent :type "PrimitiveComponent Object Reference") (OtherActor :type "Actor Object Reference") (OtherComp :type "PrimitiveComponent Object Reference") (OtherBodyIndex :type Integer) (bFromSweep :type Boolean) (SweepResult :type "HitResult Structure (by ref)"))
  ; Win Condition
  (`self.WinCondition`))

(event `WinCondition`
  (bind _returnvalue (`GameplayStatics.GetPlayerController` 0))
  ; Win Condition
  (bind _returnvalue_2 (`|CreateWidget` "/Game/Mywork/Blueprints/UI/WBP_WinMenu.WBP_WinMenu_C"))
  (`UserWidget.AddToViewport` _returnvalue_2 0)
  (set `PlayerController.bShowMouseCursor` true _returnvalue)
  (`WidgetBlueprintLibrary.SetInputMode_UIOnlyEx` _returnvalue (`self.WIDWinMenuRef`))
  (`GameplayStatics.SetGamePaused` true))

(fn `UserConstructionScript`)