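; BP_RoofRectLightFlicker is a roof rect light that flickers during play.
; The construction script sets the light to its normal intensity.
; From BeginPlay it loops on a retriggerable delay of random length between Min and Max, with a FlipFlop alternating the light between MinIntensity and Intensity on each pass.
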(event `self.ReceiveBeginPlay`
  (bind _rectlight (`self.RectLight`))
  (`KismetSystemLibrary.RetriggerableDelay` (`KismetMathLibrary.RandomFloatInRange` (`self.Min`) (`self.Max`)) :!label _label)
  (`/Engine/EditorBlueprintResources/StandardMacros.FlipFlop`
    (:`A`
      (`LightComponent.SetIntensity` _rectlight (`self.MinIntensity`))
      (goto _label))
    (:`B`
      (`LightComponent.SetIntensity` _rectlight (`self.Intensity`))
      (goto _label))))

(fn `UserConstructionScript`
  (`LightComponent.SetIntensity` (`self.RectLight`) (`self.Intensity`)))