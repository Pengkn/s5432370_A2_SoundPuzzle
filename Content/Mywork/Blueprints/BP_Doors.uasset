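; Sliding door Blueprint that opens on interaction once its WasCorrect flag, not set true in this file, unlocks it.
; Box overlaps track CloseEnough and show or remove an interact prompt widget for the player.
; Interact calls UseDoor, which plays a sound and a timeline sliding the door along local Y, clearing WasCorrect, or shows HUD text if locked.
; Camera shake and custom-depth highlighting are disabled.
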(event `UseDoor`
  (bind _hudmanagerref (`self.HUDmanagerref`))
  ;[0.15 0.08458 0.1491 0.5] Door Interaction, lock check and Animation:
  (if (`self.CloseEnough`)
    (if (`self.WasCorrect?`)
      (`GameplayStatics.PlaySound2D` "/Game/Mywork/Assets/Audios/AUD_Door.AUD_Door" 1.0 1.0 0.0 null null)
      (`GameplayStatics.PlayWorldCameraShake` "/Game/Mywork/Blueprints/BP_CameraShake.BP_CameraShake_C" (`self.K2_GetActorLocation`) 0.0 200.0 :!enabledstate Disabled)
      (bind (_direction _newtrack_0) (`Timeline|Door_open/close`)
        (:`Update`
          (`SceneComponent.K2_SetRelativeLocation` (`self.Door`) (`KismetMathLibrary.VLerp` (0.0 47.0 0.0) (0.0 115.0 0.0) _newtrack_0) false false)
          (set `self.WasCorrect?` false)))
      (else
        (`/Game/Mywork/UI/WBP_HUD.set enum` (`/Game/Mywork/Blueprints/BP_HUDManager.HUD_Ref` _hudmanagerref) "NewEnumerator6")
        (`/Game/Mywork/Blueprints/BP_HUDManager.SetHUDtextVisibility` _hudmanagerref)))))

(event `self.Box.OnComponentBeginOverlap`
  (params (OverlappedComponent :type "PrimitiveComponent Object Reference") (OtherActor :type "Actor Object Reference") (OtherComp :type "PrimitiveComponent Object Reference") (OtherBodyIndex :type Integer) (bFromSweep :type Boolean) (SweepResult :type "HitResult Structure (by ref)"))
  ;[0.15 0.1428 0.05557 0.5] InteractPrompt Widget
  (set `self.CloseEnough` true)
  (if (== OtherActor (`GameplayStatics.GetPlayerCharacter` 0))
    (`UserWidget.AddToViewport` (`self.InteractPrompt`) 0)
    (`PrimitiveComponent.SetRenderCustomDepth` (`self.Door` :!enabledstate Disabled) true :!enabledstate Disabled)))

(event `self.Box.OnComponentEndOverlap`
  (params (OverlappedComponent :type "PrimitiveComponent Object Reference") (OtherActor :type "Actor Object Reference") (OtherComp :type "PrimitiveComponent Object Reference") (OtherBodyIndex :type Integer))
  ;[0.15 0.1428 0.05557 0.5] InteractPrompt Widget
  (set `self.CloseEnough` false)
  (if (== (`GameplayStatics.GetPlayerCharacter` 0) OtherActor)
    (`Widget.RemoveFromParent` (`self.InteractPrompt`))
    (`PrimitiveComponent.SetRenderCustomDepth` (`self.Door` :!enabledstate Disabled) false :!enabledstate Disabled)))

(event `self.ReceiveBeginPlay`
  ;[0.15 0.1428 0.05557 0.5] InteractPrompt Widget
  (bind _returnvalue (`|CreateWidget` "/Game/Mywork/UI/WBP_InteractPrompt.WBP_InteractPrompt_C"))
  (set `self.InteractPrompt` _returnvalue)
  (`WidgetBlueprintLibrary.SetInputMode_GameOnly` (`GameplayStatics.GetPlayerController` 0)))

(fn `Interact`
  (params (Interactor :type "Character Object Reference"))
  (returns (Sucess :type Boolean))
  (`self.UseDoor`)
  (return false))

(fn `UserConstructionScript`)